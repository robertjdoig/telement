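; Trigger volume for the main chamber that lights braziers in staged sequence when the player enters.
; On overlap by an actor tagged Player, it calls TriggerableEvent with switch on for each brazier in three arrays, BrazierMk I, 2 and 3.
; A two-second delay separates each group, so the braziers activate in three waves.
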(event `self.ReceiveActorBeginOverlap`
  (params (OtherActor :type "Actor Object Reference"))
  (if (`self.ActorHasTag` OtherActor "Player")
    (for _array_element (`self.Brazier Mk. I`)
      (`/Game/Blueprints/Triggerable_Object/Triggerable_Object.Triggerable Event` _array_element true 0.0 0.0))
    (`KismetSystemLibrary.Delay` 2.0)
    (for _array_element_2 (`self.Brazier Mk. 2`)
      (`/Game/Blueprints/Triggerable_Object/Triggerable_Object.Triggerable Event` _array_element_2 true 0.0 0.0))
    (`KismetSystemLibrary.Delay` 2.0)
    (for _array_element_3 (`self.Brazier Mk. 3`)
      (`/Game/Blueprints/Triggerable_Object/Triggerable_Object.Triggerable Event` _array_element_3 true 0.0 0.0))))

(fn `UserConstructionScript`)