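; Spawner actor that rains out randomized Bullet actors inside its SpawnBox volume while the SpawnBall input is held.
; The input press and release open and close a gate on Tick, with a 0.1-second Delay throttling the spawn rate.
; Each spawn gets a random offset within the scaled box extent around the actor's location, plus random rotation and per-axis scale.
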(event `self.ReceiveTick`
  (params (DeltaSeconds :type "Float (single-precision)"))
  (bind _returnvalue (`KismetMathLibrary.RandomFloatInRange` 0.2 1.0))
  (bind _x (.x (`BoxComponent.GetScaledBoxExtent` (`self.SpawnBox`))))
  (bind _y (.y (`BoxComponent.GetScaledBoxExtent` (`self.SpawnBox`))))
  (bind _z (.z (`BoxComponent.GetScaledBoxExtent` (`self.SpawnBox`))))
  ;[1 1 1] Event tp Spawn Object
  (`/Engine/EditorBlueprintResources/StandardMacros.Gate` true :!label _label
    (:`Exit`
      (`KismetSystemLibrary.Delay` 0.1)
      ;[1 1 1] Spawning Object
      (`|SpawnActorFromClass` "/Game/Blueprints/Bullet.Bullet_C" (`KismetMathLibrary.MakeTransform` (+ (`KismetMathLibrary.MakeVector` (`KismetMathLibrary.RandomFloatInRange` (* _x -1.0) _x) (`KismetMathLibrary.RandomFloatInRange` (* _y -1.0) _y) (`KismetMathLibrary.RandomFloatInRange` (* _z -1.0) _z)) (`self.K2_GetActorLocation`)) (`KismetMathLibrary.RandomRotator` true) (`KismetMathLibrary.MakeVector` _returnvalue _returnvalue _returnvalue)) "Undefined" "OverrideRootScale"))))

(event `InputAction|SpawnBall`
  (params (Key :type "Key Structure" :default "AnyKey"))
  ;[1 1 1] Event tp Spawn Object
  (:`Pressed`
    (goto _label :!via `Open`))
  (:`Released`
    (goto _label :!via `Close`)))

(fn `UserConstructionScript`)