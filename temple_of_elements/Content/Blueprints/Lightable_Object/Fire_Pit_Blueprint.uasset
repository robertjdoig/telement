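; Fire pit actor that can be lit or put out according to the type of damage it receives.
; A damage event shows the particle system and plays the torch-on sound at the mesh for FireDamage, and hides the particles for FireDrainDamage.
; BeginPlay also plays the torch-on sound at double volume, with no location supplied.
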(event `CustomEvent`
  (params (Damage :type "Float (double-precision)" :default 0.0) (DamageType :type "DamageType Object Reference") (InstigatedBy :type "Controller Object Reference") (DamageCauser :type "Actor Object Reference"))
  (bind _returnvalue (`GameplayStatics.GetObjectClass` DamageType))
  (bind _particlesystem (`self.ParticleSystem`))
  (if (== _returnvalue "/Game/Blueprints/Player/Projectiles/FireDamage.FireDamage_C")
    (`SceneComponent.SetVisibility` _particlesystem true false)
    (`GameplayStatics.PlaySoundAtLocation` "/Game/Sounds/Props/torch_on_sound.torch_on_sound" (`SceneComponent.K2_GetComponentLocation` (`self.StaticMeshComponent`)))
    (elif (== _returnvalue "/Game/Blueprints/Player/Projectiles/FireDrainDamage.FireDrainDamage_C")
      (`SceneComponent.SetVisibility` _particlesystem false false))))

(event `self.ReceiveBeginPlay`
  (`GameplayStatics.PlaySoundAtLocation` "/Game/Sounds/Props/torch_on_sound.torch_on_sound" (0.0 0.0 0.0) (struct) 2.0))

(fn `UserConstructionScript`)