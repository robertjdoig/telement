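; Lightable torch object that toggles its particle effect in response to fire-related damage types.
; On AnyDamage, an exact class check hides the particle system for FireDamage and shows it for FireDrainDamage, the inverse of what those names suggest.
; Both branches then play a sound at the torch mesh's location, and other damage types are ignored.
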(event `self.ReceiveAnyDamage`
  (params (Damage :type "Float (single-precision)") (DamageType :type "DamageType Object Reference") (InstigatedBy :type "Controller Object Reference") (DamageCauser :type "Actor Object Reference"))
  (bind _returnvalue (`GameplayStatics.GetObjectClass` DamageType))
  (bind _particlesystem (`self.ParticleSystem`))
  (bind _returnvalue_2 (`SceneComponent.K2_GetComponentLocation` (`self.TorchMesh`)))
  (if (== _returnvalue "/Game/Blueprints/Player/Projectiles/FireDamage.FireDamage_C")
    (`SceneComponent.SetVisibility` _particlesystem false false)
    (`GameplayStatics.PlaySoundAtLocation` null _returnvalue_2)
    (elif (== _returnvalue "/Game/Blueprints/Player/Projectiles/FireDrainDamage.FireDrainDamage_C")
      (`SceneComponent.SetVisibility` _particlesystem true false)
      (`GameplayStatics.PlaySoundAtLocation` null _returnvalue_2))))

(fn `UserConstructionScript`)