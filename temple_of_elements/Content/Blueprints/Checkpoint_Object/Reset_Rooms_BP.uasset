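; Checkpoint room reset actor that respawns crystals at recorded urn locations when something overlaps it.
; Other objects register positions through Add_Urn_Location, which appends them to an array.
; On overlap it spawns a Crystal_Inital at each stored location, passes itself as that crystal's room reset object, then clears the array.
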(event `self.ReceiveActorBeginOverlap`
  (params (OtherActor :type "Actor Object Reference"))
  (bind _result (`/Engine/EditorBlueprintResources/StandardMacros.DecrementInt` (`KismetArrayLibrary.Array_Length` (`self.Urns_Locations`)))
    (:`  `
      (for _index (range (+ _result 1))
        (bind _returnvalue (`|SpawnActorFromClass` "/Game/Blueprints/Destructable_Object/Crystal_Urn/Crystal_Inital.Crystal_Inital_C" (`KismetMathLibrary.MakeTransform` (`KismetArrayLibrary.Array_Get` (`self.Urns_Locations`) _index)) "AdjustIfPossibleButAlwaysSpawn" "OverrideRootScale"))
        (`/Game/Blueprints/Destructable_Object/Crystal_Urn/Crystal_Inital.Set_Room_Reset_Object` _returnvalue self))
      (`KismetArrayLibrary.Array_Clear` (`self.Urns_Locations`)))))

(event `Add_Urn_Location`
  (params (NewParam :type "Vector Structure"))
  (`KismetArrayLibrary.Array_Add` (`self.Urns_Locations`) NewParam))

(fn `UserConstructionScript`)