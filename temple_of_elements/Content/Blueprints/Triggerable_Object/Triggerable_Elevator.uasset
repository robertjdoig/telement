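; Triggerable elevator actor that toggles between two positions each time its TriggerableEvent fires.
; It caches its starting location at BeginPlay and uses the ShouldGoDown flag to alternate between playing and reversing a timeline.
; The timeline's Movement output is added to that starting location to set the actor's position, without sweep.
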(event `self.ReceiveBeginPlay`
  (set `self.Initial location` (`self.K2_GetActorLocation`)))

(event `self.Triggerable Event`
  (params (`Switch State` :type Boolean) (Value :type "Float (single-precision)") (Delay :type "Float (single-precision)"))
  (if (`self.Should Go Down`)
    (set `self.Should Go Down` false)
    (bind (_direction _movement) (`Timeline|Timeline_0` :!label _label)
      (:`Update`
        (`self.K2_SetActorLocation` (+ (`self.Initial location`) _movement))))
    (else
      (set `self.Should Go Down` true)
      (goto _label :!via `Reverse`))))

(fn `UserConstructionScript`
  (`parent.UserConstructionScript`))