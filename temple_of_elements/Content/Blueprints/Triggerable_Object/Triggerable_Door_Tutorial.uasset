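; Triggerable tutorial door that slides vertically between open and closed and can be destroyed by heavy damage.
; A trigger waits for a delay, plays a stone sound at world origin, then flips IsClosed and plays or reverses a timeline driving the door's Z.
; BeginPlay pre-inverts the flag and runs the same toggle to apply the initial state.
; Heavy hits feed a countdown check that swaps in a destruct actor with a pottery sound.
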(event `self.ReceiveBeginPlay`
  (if (`self.IsClosed`)
    (set `self.IsClosed` false)
    (else
      (set `self.IsClosed` true)))
  (if (`self.IsClosed`) :!label _label
    (set `self.IsClosed` false)
    (bind (_direction _doorposition) (`Timeline|Timeline_0` :!label _label_2)
      (:`Update`
        (`SceneComponent.K2_SetRelativeLocation` (`self.Door`) (`KismetMathLibrary.MakeVector` 0.0 0.0 _doorposition) false false)))
    (else
      (set `self.IsClosed` true)
      (goto _label_2 :!via `Reverse`))))

(event `self.Triggerable Event`
  (params (`Switch State` :type Boolean) (Value :type "Float (single-precision)") (Delay :type "Float (single-precision)"))
  (`KismetSystemLibrary.Delay` Delay)
  (`GameplayStatics.SpawnSoundAtLocation` "/Game/Sounds/Props/Stone_door.Stone_door")
  (goto _label))

(event `self.ReceiveAnyDamage`
  (params (Damage :type "Float (single-precision)") (DamageType :type "DamageType Object Reference") (InstigatedBy :type "Controller Object Reference") (DamageCauser :type "Actor Object Reference"))
  (bind (_returnvalue_location _returnvalue_rotation) (`KismetMathLibrary.BreakTransform` (`SceneComponent.K2_GetComponentToWorld` (`self.DefaultSceneRoot`))))
  (if (> Damage 99.0)
    (bind _output_get (set `self.Damage` (- (`self.Damage`) 1)))
    (if (< _output_get 1)
      (`|SpawnActorFromClass` "/Game/Blueprints/Destructable_Object/Crystal_Urn/Door_Destruct.Door_Destruct_C" (`KismetMathLibrary.MakeTransform` _returnvalue_location _returnvalue_rotation (0.7 0.9 1.0)) "AdjustIfPossibleButAlwaysSpawn" "OverrideRootScale")
      (`GameplayStatics.PlaySoundAtLocation` "/Game/Sounds/Props/pottery.pottery" _returnvalue_location)
      (`self.K2_DestroyActor`))))

(fn `UserConstructionScript`
  (`parent.UserConstructionScript`))