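; A triggerable spike trap that damages whatever it hits and guards a lever.
; When triggered, it plays a spike sound and runs a timeline that offsets the actor from its starting location, with an event track replaying the sound.
; When the timeline finishes, it unlocks the protected lever.
; Hits apply fixed damage to the other actor and spawn an impact effect at the hit location.
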(event `self.ReceiveBeginPlay`
  (set `self.Initial location` (`self.K2_GetActorLocation`)))

(event `self.Triggerable Event`
  (params (`Switch State` :type Boolean) (Value :type "Float (single-precision)") (Delay :type "Float (single-precision)"))
  (`GameplayStatics.SpawnSoundAtLocation` "/Game/Sounds/Props/spikes.spikes" (`SceneComponent.K2_GetComponentLocation` (`self.StaticMesh`)))
  (bind (_direction _movement) (`Timeline|Timeline_0` :!via `PlayFromStart`)
    (:`Update`
      (`self.K2_SetActorLocation` (+ (`self.Initial location`) _movement)))
    (:`Finished`
      (set `/Game/Blueprints/Triggerable_Object/Triggers/Lever.Unlocked` true (`self.Protected lever`)))
    (:`Play sound`
      (`GameplayStatics.PlaySoundAtLocation` "/Game/Sounds/Props/spikes.spikes" (`SceneComponent.K2_GetComponentLocation` (`self.DefaultSceneRoot`))))))

(event `self.ReceiveHit`
  (params (MyComp :type "PrimitiveComponent Object Reference") (Other :type "Actor Object Reference") (OtherComp :type "PrimitiveComponent Object Reference") (bSelfMoved :type Boolean) (HitLocation :type "Vector Structure") (HitNormal :type "Vector Structure") (NormalImpulse :type "Vector Structure") (Hit :type "HitResult Structure (by ref)"))
  (`GameplayStatics.ApplyDamage` Other 6.0)
  (`|SpawnActorFromClass` "/Game/Blueprints/Spawner/Bullets/Spike_hit_effect.Spike_hit_effect_C" (`KismetMathLibrary.MakeTransform` HitLocation) "Undefined" "OverrideRootScale"))

(fn `UserConstructionScript`
  (`parent.UserConstructionScript`))