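; Triggerable rising bridge that toggles between two positions when its trigger event fires.
; TriggerableEvent waits for Delay, plays a stone door sound at the world origin, then plays or reverses the MoveBlock timeline according to IsDown.
; The timeline offsets the actor in Y and Z from the location stored at BeginPlay.
; BeginPlay flips IsDown and runs the same toggle, driving the timeline to match the initial flag.
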(event `self.ReceiveBeginPlay`
  (bind (_initial_position_x _initial_position_y _initial_position_z) (`KismetMathLibrary.BreakVector` (`self.Initial Position`)))
  (set `self.Initial Position` (`self.K2_GetActorLocation`))
  (if (`self.Is Down`)
    (set `self.Is Down` false)
    (else
      (set `self.Is Down` true)))
  (if (`self.Is Down`) :!label _label
    (set `self.Is Down` false)
    (bind (_direction _block_y_position _block_z_positio) (`Timeline|Move Block` :!label _label_2)
      (:`Update`
        (`self.K2_SetActorRelativeLocation` (`KismetMathLibrary.MakeVector` _initial_position_x (+ _initial_position_y _block_y_position) (+ _initial_position_z _block_z_positio)))))
    (else
      (set `self.Is Down` true)
      (goto _label_2 :!via `Reverse`))))

(event `self.Triggerable Event`
  (params (`Switch State` :type Boolean) (Value :type "Float (single-precision)") (Delay :type "Float (single-precision)"))
  (`KismetSystemLibrary.Delay` (`self.Delay`))
  (`GameplayStatics.SpawnSoundAtLocation` "/Game/Sounds/Props/Stone_door.Stone_door")
  (goto _label))

(fn `UserConstructionScript`
  (`parent.UserConstructionScript`))