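; A triggerable floor piece that rises or lowers by sliding its static mesh along relative Z.
; An IsDown flag selects whether a timeline plays or reverses, flipping each time.
; BeginPlay inverts the flag and runs that toggle to set the starting state.
; TriggerableEvent waits for the given delay, spawns a stone door sound at the world origin, then runs the same toggle.
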(event `self.ReceiveBeginPlay`
  (if (`self.Is Down`)
    (set `self.Is Down` false)
    (else
      (set `self.Is Down` true)))
  (if (`self.Is Down`) :!label _label
    (set `self.Is Down` false)
    (bind (_direction _doorposition) (`Timeline|Timeline_0` :!label _label_2)
      (:`Update`
        (`SceneComponent.K2_SetRelativeLocation` (`self.StaticMesh`) (`KismetMathLibrary.MakeVector` 0.0 0.0 _doorposition) false false)))
    (else
      (set `self.Is Down` true)
      (goto _label_2 :!via `Reverse`))))

(event `self.Triggerable Event`
  (params (`Switch State` :type Boolean) (Value :type "Float (single-precision)") (Delay :type "Float (single-precision)"))
  (`KismetSystemLibrary.Delay` Delay)
  (`GameplayStatics.SpawnSoundAtLocation` "/Game/Sounds/Props/Stone_door.Stone_door")
  (goto _label))

(fn `UserConstructionScript`
  (`parent.UserConstructionScript`))