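; Triggerable object with a crystal that gives the player the element device and can launch a fire bullet.
; Any damage lights the crystal and stops the side fire spawner.
; When triggered while lit, it waits, fires a gravity-free bullet near its arrow, destroys the crystal and triggers FIXERTorch.
; A hit from the player enables the back spawner, activates the character's element device and destroys the actor.
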(event `self.ReceiveAnyDamage`
  (params (Damage :type "Float (single-precision)") (DamageType :type "DamageType Object Reference") (InstigatedBy :type "Controller Object Reference") (DamageCauser :type "Actor Object Reference"))
  (`PrimitiveComponent.SetMaterial` (`self.Crystal`) 0 "/Game/Levels/Air_level/Materials/Glow1_M.Glow1_M")
  (set `/Game/Blueprints/Spawner/wall_spawner_fire.Should Spawn` false (`self.FireSpawnerSide`))
  (set `self.Crystal Lit` true))

(event `self.Triggerable Event`
  (params (`Switch State` :type Boolean) (Value :type "Float (single-precision)") (Delay :type "Float (single-precision)"))
  (bind _returnvalue (`SceneComponent.K2_GetComponentRotation` (`self.DefaultSceneRoot`)))
  (if (`self.Crystal Lit`)
    (set `self.Crystal Lit` false)
    (`KismetSystemLibrary.Delay` 5.0)
    (bind _returnvalue_2 (`|SpawnActorFromClass` "/Game/Blueprints/Spawner/Bullets/Fire_Bullet.Fire_bullet_C" (`KismetMathLibrary.MakeTransform` (+ (`SceneComponent.K2_GetComponentLocation` (`self.Arrow`)) (`KismetMathLibrary.GreaterGreater_VectorRotator` (0.0 0.0 0.0) _returnvalue) (-50.0 0.0 0.0)) _returnvalue) "AlwaysSpawn" "OverrideRootScale"))
    (`/Game/Blueprints/Spawner/Bullets/Fire_Bullet.SetBulletGravity` _returnvalue_2 0.0)
    (`ActorComponent.K2_DestroyComponent` (`self.Crystal`))
    (`self.Triggerable Event` (`self.FIXER_Torch`) true 0.0 0.0)))

(event `self.ReceiveHit`
  (params (MyComp :type "PrimitiveComponent Object Reference") (Other :type "Actor Object Reference") (OtherComp :type "PrimitiveComponent Object Reference") (bSelfMoved :type Boolean) (HitLocation :type "Vector Structure") (HitNormal :type "Vector Structure") (NormalImpulse :type "Vector Structure") (Hit :type "HitResult Structure (by ref)"))
  (if (`self.ActorHasTag` Other "Player")
    (`KismetSystemLibrary.PrintString` "Element Device Activated") ; TURN ON THE GUN GUI
    (set `/Game/Blueprints/Spawner/wall_spawner_fire.Should Spawn` true (`self.FireSpawnerBack`))
    (bind _asfirst_person_character (cast `/Game/Blueprints/Player/FirstPersonCharacter` (`GameplayStatics.GetPlayerCharacter` 0)))
    (`/Game/Blueprints/Player/FirstPersonCharacter.Activate Element Device` _asfirst_person_character)
    (`self.K2_DestroyActor`)))

(fn `UserConstructionScript`
  (`parent.UserConstructionScript`))