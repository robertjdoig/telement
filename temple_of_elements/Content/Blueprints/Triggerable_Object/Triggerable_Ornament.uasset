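; Triggerable ornament actor that hovers and spins, and whose Ornament component can be revealed by a trigger.
; BeginPlay caches the initial transform, then a timeline drives a Z offset and absolute yaw from that base.
; TriggerableEvent makes the Ornament visible.
; When StartVisible is false, every timeline update hides it again, so a reveal is overridden while the timeline plays.
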(event `self.Triggerable Event`
  (params (`Switch State` :type Boolean) (Value :type "Float (single-precision)") (Delay :type "Float (single-precision)"))
  (`SceneComponent.SetVisibility` (`self.Ornament`) true false))

(event `self.ReceiveBeginPlay`
  (bind _initial_transform (`self.Initial transform`))
  (set `self.Initial transform` (`self.GetTransform`))
  (bind (_direction _rotate _hover) (`Timeline|Timeline_0`)
    (:`Update`
      (`self.K2_SetActorLocationAndRotation` (`KismetMathLibrary.MakeVector` (.x (.location _initial_transform)) (.y (.location _initial_transform)) (+ _hover (.z (.location (`self.Initial transform`))))) (`KismetMathLibrary.MakeRotator` (.roll (.rotation _initial_transform)) (.pitch (.rotation _initial_transform)) _rotate))
      (if (not (`self.Start visible`))
        (`SceneComponent.SetVisibility` (`self.Ornament`) false false)))))

(fn `UserConstructionScript`
  (`parent.UserConstructionScript`))