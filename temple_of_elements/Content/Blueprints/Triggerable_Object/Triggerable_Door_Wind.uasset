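; Triggerable stone door that slides vertically when it receives a switch event.
; After the event's delay, it plays a door sound at the world origin and stores its current location as the base.
; A timeline plays from start when switched on and reverses when off, setting the actor's Z to that base plus the curve value.
; The base is re-captured on every trigger, including reversals.
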(event `self.Triggerable Event`
  (params (`Switch State` :type Boolean) (Value :type "Float (single-precision)") (Delay :type "Float (single-precision)"))
  (bind (_returnvalue_x _returnvalue_y) (`KismetMathLibrary.BreakVector` (`self.K2_GetActorLocation`)))
  (bind (_initial_location_x _initial_location_y _initial_location_z) (`KismetMathLibrary.BreakVector` (`self.Initial Location`)))
  (`KismetSystemLibrary.Delay` Delay)
  (`GameplayStatics.SpawnSoundAtLocation` "/Game/Sounds/Props/Stone_door.Stone_door")
  (set `self.Initial Location` (`self.K2_GetActorLocation`))
  (if `Switch State`
    (bind (_direction _doorposition) (`Timeline|Timeline_0` :!via `PlayFromStart` :!label _label)
      (:`Update`
        (`self.K2_SetActorLocation` (`KismetMathLibrary.MakeVector` _returnvalue_x _returnvalue_y (+ _doorposition _initial_location_z)))))
    (else
      (goto _label :!via `Reverse`))))

(fn `UserConstructionScript`
  (`parent.UserConstructionScript`))