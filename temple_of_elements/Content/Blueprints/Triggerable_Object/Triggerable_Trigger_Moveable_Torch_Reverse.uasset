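; Triggerable torch that fire damage lights and fire-drain damage extinguishes, firing separate lists of triggerables for each change.
; TriggerableEvent switches it too; a non-zero Value skips the triggers and IsLit update, changing only particles and lighting sound.
; BeginPlay stores the location and always ends up reversing the Y/Z movement timeline, as IsDown is forced false first.
; Logic syncing particles to the initial IsLit is disconnected.
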(event `self.ReceiveAnyDamage`
  (params (Damage :type "Float (single-precision)") (DamageType :type "DamageType Object Reference") (InstigatedBy :type "Controller Object Reference") (DamageCauser :type "Actor Object Reference"))
  (bind _returnvalue (`GameplayStatics.GetObjectClass` DamageType))
  (if (== _returnvalue "/Game/Blueprints/Player/Projectiles/FireDamage.FireDamage_C")
    (for _array_element (`self.Triggers When Lit`) :!label _label
      (`self.Triggerable Event` _array_element true 0.0 0.0))
    (set `self.Is Lit` true)
    (`SceneComponent.SetVisibility` (`self.ParticleSystem`) true false :!label _label_2)
    (`GameplayStatics.PlaySoundAtLocation` "/Game/Sounds/Props/torch_on_sound.torch_on_sound" (`SceneComponent.K2_GetComponentLocation` (`self.Torch Mesh`)))
    (elif (== _returnvalue "/Game/Blueprints/Player/Projectiles/FireDrainDamage.FireDrainDamage_C")
      (for _array_element_2 (`self.Triggers When Extinguished`) :!label _label_3
        (`self.Triggerable Event` _array_element_2 false 0.0 0.0))
      (set `self.Is Lit` false)
      (`SceneComponent.SetVisibility` (`self.ParticleSystem`) false false :!label _label_4))))

(event `self.Triggerable Event`
  (params (`Switch State` :type Boolean) (Value :type "Float (single-precision)") (Delay :type "Float (single-precision)"))
  (if (== Value 0.0)
    (if `Switch State`
      (goto _label)
      (else
        (goto _label_3)))
    (elif `Switch State`
      (goto _label_2)
      (else
        (goto _label_4)))))

(event `self.ReceiveBeginPlay`
  (bind (_initial_position_x _initial_position_y _initial_position_z) (`KismetMathLibrary.BreakVector` (`self.Initial Position`)))
  (set `self.Initial Position` (`self.K2_GetActorLocation`))
  (if (`self.Is Down`)
    (set `self.Is Down` false)
    (else
      (set `self.Is Down` false)))
  (if (`self.Is Down`)
    (set `self.Is Down` false)
    (bind (_direction _block_y_position _block_z_positio) (`Timeline|Timeline_0` :!label _label_5)
      (:`Update`
        (`self.K2_SetActorRelativeLocation` (`KismetMathLibrary.MakeVector` _initial_position_x (+ _initial_position_y _block_y_position) (+ _initial_position_z _block_z_positio)))))
    (else
      (set `self.Is Down` true)
      (goto _label_5 :!via `Reverse`))))

(fn `UserConstructionScript`
  (`parent.UserConstructionScript`))