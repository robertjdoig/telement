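; A triggerable physics wall that shuttles back and forth along Y between its start position and a maximum distance.
; From BeginPlay, two timelines alternately push the mesh with AddForce, zeroing its linear and angular velocity at each limit before reversing, while Tick stops the inactive timeline.
; The trigger event toggles a slow flag that Tick turns into ForceOfPush, but the AddForce calls use a hard-coded multiplier instead.
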(event `self.ReceiveBeginPlay`
  (bind _staticmesh (`self.StaticMesh`))
  (bind _staticmesh_2 (`self.StaticMesh`))
  (bind (_relativelocation_x _relativelocation_y) (`KismetMathLibrary.BreakVector` (`SceneComponent.RelativeLocation` (`self.StaticMesh`))))
  (bind _output_get (set `self.Initial Location` (`SceneComponent.RelativeLocation` (`self.StaticMesh`))))
  (bind (_direction _movement) (`Timeline|Timeline_0` :!via `PlayFromStart` :!label _label) ; Forwards
    (:`Update`
      (bind _y (.y _output_get))
      (if (> _relativelocation_y (+ _y (`self.Max Distance Y`)))
        (`PrimitiveComponent.SetPhysicsLinearVelocity` _staticmesh_2 (0.0 0.0 0.0) false "None")
        (`PrimitiveComponent.SetPhysicsAngularVelocity` _staticmesh_2 (0.0 0.0 0.0) false "None")
        (set `self.Move Forwards` false)
        (bind (_direction_2 _movement_2) (`Timeline|Timeline_1` :!via `PlayFromStart` :!label _label_2)
          (:`Update`
            (if (< _relativelocation_y _y)
              (`PrimitiveComponent.SetPhysicsLinearVelocity` _staticmesh_2 (0.0 0.0 0.0) false "None")
              (`PrimitiveComponent.SetPhysicsAngularVelocity` _staticmesh_2 (0.0 0.0 0.0) false "None")
              (set `self.Move Forwards` true)
              (goto _label :!via `PlayFromStart`)
              (else
                (`PrimitiveComponent.AddForce` _staticmesh (* _movement_2 100000.0) "None" false)))))
        (else
          (`PrimitiveComponent.AddForce` _staticmesh (* _movement 100000.0) "None" false))))))

(event `self.ReceiveTick`
  (params (DeltaSeconds :type "Float (single-precision)"))
  (if (`self.Should Go Slow`)
    (set `self.Force Of Push` 10000.0)
    (else
      (set `self.Force Of Push` 100000.0)))
  (if (`self.Move Forwards`)
    (goto _label_2 :!via `Stop`)
    (else
      (goto _label :!via `Stop`))))

(event `self.Triggerable Event`
  (params (`Switch State` :type Boolean) (Value :type "Float (single-precision)") (Delay :type "Float (single-precision)"))
  (set `self.Should Go Slow` `Switch State`))

(fn `UserConstructionScript`
  (`parent.UserConstructionScript`))