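; Triggerable fire pit that lights on fire damage and goes out on fire-drain damage, firing other triggerables on each change.
; Incoming TriggerableEvents drive the same paths by SwitchState; a non-zero Value skips the chained triggers and IsLit update, changing only the effects.
; Lighting shows the particle system and plays a torch sound, extinguishing hides the particles, and BeginPlay applies the effects matching IsLit.
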(event `self.ReceiveAnyDamage`
  (params (Damage :type "Float (single-precision)") (DamageType :type "DamageType Object Reference") (InstigatedBy :type "Controller Object Reference") (DamageCauser :type "Actor Object Reference"))
  (bind _returnvalue (`GameplayStatics.GetObjectClass` DamageType))
  (if (== _returnvalue "/Game/Blueprints/Player/Projectiles/FireDamage.FireDamage_C")
    (for _array_element _ :!label _label
      (`self.Triggerable Event` _array_element false 0.0 0.0))
    (set `self.Is Lit` true)
    (`SceneComponent.SetVisibility` (`self.ParticleSystem`) true false :!label _label_2)
    (`GameplayStatics.PlaySoundAtLocation` "/Game/Sounds/Props/torch_on_sound.torch_on_sound" (`SceneComponent.K2_GetComponentLocation` (`self.Fire Pit Mesh`)))
    (elif (== _returnvalue "/Game/Blueprints/Player/Projectiles/FireDrainDamage.FireDrainDamage_C")
      (for _array_element_2 (`self.Triggers When Extinguished`) :!label _label_3
        (`self.Triggerable Event` _array_element_2 false 0.0 0.0))
      (set `self.Is Lit` false)
      (`SceneComponent.SetVisibility` (`self.ParticleSystem`) false false :!label _label_4))))

(event `self.Triggerable Event`
  (params (`Switch State` :type Boolean) (Value :type "Float (single-precision)") (Delay :type "Float (single-precision)"))
  (if (== Value 0.0)
    (if `Switch State`
      (goto _label)
      (else
        (goto _label_3)))
    (elif `Switch State`
      (goto _label_2)
      (else
        (goto _label_4)))))

(event `self.ReceiveBeginPlay`
  (if (`self.Is Lit`)
    (goto _label_2)
    (else
      (goto _label_4))))

(fn `UserConstructionScript`
  (`parent.UserConstructionScript`))