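; Fire_Spawner is a spawner actor that repeatedly fires Fire_bullet actors while its ShouldSpawn flag is on.
; Tick runs a short Delay to pace the spawn rate, then rechecks the flag before spawning.
; Each bullet appears at the SpawnLocation component with the root's rotation, ignoring collisions, and receives the spawner's BulletGravity.
; The rotated forward offset is zero, so it leaves the position unchanged.
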(event `self.ReceiveTick`
  (params (DeltaSeconds :type "Float (single-precision)"))
  (bind _returnvalue (`SceneComponent.K2_GetComponentRotation` (`self.DefaultSceneRoot`)))
  ;[1 1 1] Event to Spawn Object
  (if (`self.ShouldSpawn`)
    ;;[1 1 1] Spawn Rate
    (`KismetSystemLibrary.Delay` 0.5)
    (if (`self.ShouldSpawn`)
      ;[1 1 1] Spawning Object
      (bind _returnvalue_2 (`|SpawnActorFromClass` "/Game/Blueprints/Spawner/Bullets/Fire_Bullet.Fire_bullet_C" (`KismetMathLibrary.MakeTransform` (+ (`SceneComponent.K2_GetComponentLocation` (`self.SpawnLocation`)) (`KismetMathLibrary.GreaterGreater_VectorRotator` (0.0 0.0 0.0) _returnvalue)) _returnvalue) "AlwaysSpawn" "OverrideRootScale"))
      (`/Game/Blueprints/Spawner/Bullets/Fire_Bullet.SetBulletGravity` _returnvalue_2 (`self.BulletGravity`)))))

(fn `UserConstructionScript`)