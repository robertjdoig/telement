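; A wall-mounted tutorial spawner actor that repeatedly fires tutorial fire bullets.
; From BeginPlay an endless delay loop waits between shots and, while ShouldSpawn is true, spawns a bullet at SpawnLocation facing along the root's rotation.
; Each bullet receives the spawner's gravity setting, and an attenuated firing sound plays at the spawner mesh.
; The forward spawn offset is a zero vector, so bullets appear exactly at SpawnLocation.
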(event `self.ReceiveBeginPlay`
  (bind _returnvalue (`SceneComponent.K2_GetComponentRotation` (`self.DefaultSceneRoot`)))
  ;[1 1 1] Event to Spawn Object
  (`KismetSystemLibrary.Delay` (`self.Bulet Delay Between Shots`) :!label _label)
  (if (`self.Should Spawn`)
    ;[1 1 1] Spawning Object
    (bind _returnvalue_2 (`|SpawnActorFromClass` "/Game/Blueprints/Spawner/Bullets/Fire_bullet_tutorial.Fire_bullet_tutorial_C" (`KismetMathLibrary.MakeTransform` (+ (`SceneComponent.K2_GetComponentLocation` (`self.SpawnLocation`)) (`KismetMathLibrary.GreaterGreater_VectorRotator` (0.0 0.0 0.0) _returnvalue)) _returnvalue) "AlwaysSpawn" "OverrideRootScale"))
    (`/Game/Blueprints/Spawner/Bullets/Fire_bullet_tutorial.SetBulletGravity` _returnvalue_2 (`self.Bullet_Gravity`))
    (`GameplayStatics.SpawnSoundAtLocation` "/Game/Sounds/Spawner/SpawnerFire.SpawnerFire" (`SceneComponent.K2_GetComponentLocation` (`self.SpawnerMesh`)) (struct) 100.0 0.0 0.0 "/Game/Sounds/Spawner/Spawner.Spawner")
    (goto _label)
    (else
      (goto _label))))

(fn `UserConstructionScript`)