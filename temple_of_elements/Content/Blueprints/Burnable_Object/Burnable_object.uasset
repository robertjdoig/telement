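; Burnable object actor that catches fire and is destroyed when hit by a Fire_Projectile_Out.
; The hit opens a gate on Tick, whose first pass sets Burning, spawns a Fire_HitEffect and starts a short delay before destroying the actor.
; Later ticks shrink the placeholder Cube by a fixed factor per frame, so the shrink speed depends on frame rate.
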(event `self.ReceiveTick`
  (params (DeltaSeconds :type "Float (single-precision)"))
  (bind _cube (`self.Cube`))
  (`/Engine/EditorBlueprintResources/StandardMacros.Gate` true :!label _label
    (:`Exit`
      (if (`self.Burning`)
        (`SceneComponent.SetWorldScale3D` _cube (* (`SceneComponent.K2_GetComponentScale` _cube) 0.99))
        (else
          (set `self.Burning` true)
          (`|SpawnActorFromClass` "/Game/Blueprints/Player/Projectiles/Fire_HitEffect.Fire_HitEffect_C" (`self.GetTransform` self) "Undefined" "OverrideRootScale")
          (`KismetSystemLibrary.Delay` 3.25)
          (`self.K2_DestroyActor`))))))

(event `self.ReceiveHit`
  (params (MyComp :type "PrimitiveComponent Object Reference") (Other :type "Actor Object Reference") (OtherComp :type "PrimitiveComponent Object Reference") (bSelfMoved :type Boolean) (HitLocation :type "Vector Structure") (HitNormal :type "Vector Structure") (NormalImpulse :type "Vector Structure") (Hit :type "HitResult Structure (by ref)"))
  (if (== (`GameplayStatics.GetObjectClass` Other) "/Game/Blueprints/Player/Projectiles/Fire_Projectile_Out.Fire_Projectile_Out_C")
    (goto _label :!via `Open`)))

(fn `UserConstructionScript`)