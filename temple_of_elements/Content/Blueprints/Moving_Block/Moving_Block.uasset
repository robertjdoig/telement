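; Moving_Block is an unfinished moving-wall actor meant to slide toward an end position over a fixed time.
; Tick lerps between the relative transforms of WallMeshProxy and EndPosition by game time over duration, applying the result as the actor transform.
; A non-looping MultiGate limits that move to a single execution rather than every frame.
; BeginPlay holds an empty, endless while loop, and a FlipFlop is left unconnected.
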(event `self.ReceiveTick`
  (params (DeltaSeconds :type "Float (single-precision)"))
  (`|MultiGate` false
    (:`Out 1`
      ;[1 1 1] Constant movement on timer
      (if true
        (`self.K2_SetActorTransform` (`KismetMathLibrary.TLerp` (`SceneComponent.GetRelativeTransform` (`self.Wall_Mesh_proxy`)) (`SceneComponent.GetRelativeTransform` (`self.End_Position`)) (`KismetMathLibrary.TimespanRatio` (- (`KismetMathLibrary.FromSeconds` (`GameplayStatics.GetTimeSeconds`)) (`KismetMathLibrary.FromSeconds` 0.0)) (`KismetMathLibrary.FromSeconds` 3.0))))))))

(event `self.ReceiveBeginPlay`
  (while true
    _))

(fn `UserConstructionScript`)