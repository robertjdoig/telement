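; Element key teleporter pad that warps the player to a linked endpoint and updates elemental quest state.
; Player overlap plays sound and particle feedback, disables input, then after a short delay hides the pad, teleports the pawn and signals KeyToTurnOn.
; The player's height after arrival determines whether the character's water or wind quest flag is cleared.
; End overlap is unwired, so stepping off does not cancel the teleport.
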(event `self.ReceiveActorEndOverlap`
  (params (OtherActor :type "Actor Object Reference")))

(event `self.ReceiveActorBeginOverlap`
  (params (OtherActor :type "Actor Object Reference"))
  (bind (_returnvalue_x _returnvalue_y _returnvalue_z) (`KismetMathLibrary.BreakVector` (`self.K2_GetActorLocation` (`GameplayStatics.GetPlayerPawn` 0))))
  (bind _returnvalue (`SceneComponent.K2_GetComponentLocation` (`self.Teleport pad`)))
  (bind (_returnvalue_location _returnvalue_rotation) (`KismetMathLibrary.BreakTransform` (`SceneComponent.K2_GetComponentToWorld` (`/Game/Blueprints/Teleporter/Teleport_End_Point.DefaultSceneRoot` (`self.Teleport End Point`)))))
  (bind _returnvalue_2 (+ _returnvalue_location (0.0 0.0 140.0)))
  (if (`self.ActorHasTag` OtherActor "Player")
    (`GameplayStatics.PlaySoundAtLocation` null _returnvalue) ; Reving up of teleporter player feedback
    (bind _returnvalue_3 (`|SpawnActorFromClass` "/Game/Blueprints/Player/Projectiles/Water_Hit_Effect.Water_Hit_Effect_C" (`KismetMathLibrary.MakeTransform` _returnvalue (struct :`Pitch` 90.0) (1.0 1.0 1.0)) "DontSpawnIfColliding" "OverrideRootScale")) ; Cool teleport particles player feedback
    (set `self.IsOnTeleporter` true)
    (`self.DisableInput` null)
    (`KismetSystemLibrary.Delay` 1.5)
    (`self.K2_DestroyActor` _returnvalue_3)
    (if (`self.IsOnTeleporter`)
      (`SceneComponent.SetVisibility` (`self.Teleport pad`) false false)
      (`self.K2_SetActorTransform` (`GameplayStatics.GetPlayerPawn` 0) (`KismetMathLibrary.MakeTransform` _returnvalue_2 _returnvalue_rotation) false true)
      (`GameplayStatics.PlaySoundAtLocation` "/Game/Sounds/Warp.Warp" _returnvalue_2) ; Teleport sound
      (`/Game/Blueprints/Triggerable_Object/Triggerable_Object.Triggerable Event` (`self.Key to Turn On`) false 0.0 0.0)
      (`self.EnableInput` null)
      (if (<= _returnvalue_z -3000.0)
        (bind _asfirst_person_character (cast `/Game/Blueprints/Player/FirstPersonCharacter` (`GameplayStatics.GetPlayerCharacter` 0)))
        (set `/Game/Blueprints/Player/FirstPersonCharacter.is_quest_water` false _asfirst_person_character)
        (else
          (bind _asfirst_person_character_2 (cast `/Game/Blueprints/Player/FirstPersonCharacter` (`GameplayStatics.GetPlayerCharacter` 0)))
          (set `/Game/Blueprints/Player/FirstPersonCharacter.is_quest_wind` false _asfirst_person_character_2))))))

(fn `UserConstructionScript`)