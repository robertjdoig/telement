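; Wind_Key is a teleporter that moves the player from its TeleportPad to its DestinationPad.
; An overlap by a Player-tagged actor plays a sound and spawns a temporary Water_Hit_Effect during a short charge-up delay.
; If the IsOnTeleporter flag survives the delay, player pawn 0 takes the destination's rotation and a raised location, with an arrival sound.
; Any actor ending overlap clears the flag, cancelling a pending teleport.
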(event `self.ReceiveActorEndOverlap`
  (params (OtherActor :type "Actor Object Reference"))
  (set `self.IsOnTeleporter` false))

(event `self.ReceiveActorBeginOverlap`
  (params (OtherActor :type "Actor Object Reference"))
  (bind (_returnvalue_location _returnvalue_rotation) (`KismetMathLibrary.BreakTransform` (`SceneComponent.K2_GetComponentToWorld` (`self.Destination pad`))))
  (bind _returnvalue (`SceneComponent.K2_GetComponentLocation` (`self.Teleport pad`)))
  (bind _returnvalue_2 (+ _returnvalue_location (0.0 0.0 140.0)))
  (if (`self.ActorHasTag` OtherActor "Player")
    (`GameplayStatics.PlaySoundAtLocation` null _returnvalue) ; Reving up of teleporter player feedback
    (bind _returnvalue_3 (`|SpawnActorFromClass` "/Game/Blueprints/Player/Projectiles/Water_Hit_Effect.Water_Hit_Effect_C" (`KismetMathLibrary.MakeTransform` _returnvalue (struct :`Pitch` 90.0) (1.0 1.0 1.0)) "DontSpawnIfColliding" "OverrideRootScale")) ; Cool teleport particles player feedback
    (set `self.IsOnTeleporter` true)
    (`KismetSystemLibrary.Delay` 1.5)
    (`self.K2_DestroyActor` _returnvalue_3)
    (if (`self.IsOnTeleporter`)
      (`self.K2_SetActorTransform` (`GameplayStatics.GetPlayerPawn` 0) (`KismetMathLibrary.MakeTransform` _returnvalue_2 _returnvalue_rotation) false true)
      (`GameplayStatics.PlaySoundAtLocation` null _returnvalue_2) ; Teleport sound
    )))

(fn `UserConstructionScript`)