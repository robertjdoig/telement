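; Resizable water block that the player can fill or drain and that drowns overlapping actors.
; Water_Projectile_Out hits raise it and WaterDrainDamage lowers it, using timelines that offset actor Z scale from its starting value, clamped to MaxSize and MinSize.
; Attempts at either limit notify FirstPersonCharacter of the failure instead.
; Overlap starts a delayed loop that repeatedly applies heavy damage while the shared IsDrowning flag stays set.
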(event `self.Water.OnComponentHit`
  (params (HitComponent :type "PrimitiveComponent Object Reference") (OtherActor :type "Actor Object Reference") (OtherComp :type "PrimitiveComponent Object Reference") (NormalImpulse :type "Vector Structure") (Hit :type "HitResult Structure (by ref)"))
  (bind (_returnvalue_x _returnvalue_y _returnvalue_z) (`KismetMathLibrary.BreakVector` (`SceneComponent.K2_GetComponentScale` (`self.Water`))))
  (bind (_returnvalue_x_2 _returnvalue_y_2) (`KismetMathLibrary.BreakVector` (`SceneComponent.K2_GetComponentScale` (`self.Water`))))
  (bind (_returnvalue_x_3 _returnvalue_y_3) (`KismetMathLibrary.BreakVector` (`SceneComponent.K2_GetComponentScale` (`self.Water`))))
  (bind (_returnvalue_x_4 _returnvalue_y_4 _returnvalue_z_2) (`KismetMathLibrary.BreakVector` (`SceneComponent.K2_GetComponentScale` (`self.Water`))))
  ;[1 1 1] Add Water
  (if (== (`GameplayStatics.GetObjectClass` OtherActor) "/Game/Blueprints/Player/Projectiles/Water_Projectile_Out.Water_Projectile_Out_C")
    (if (`KismetMathLibrary.NearlyEqual_FloatFloat` (`self.Max_Size`) _returnvalue_z_2 0.1)
      (bind _asfirst_person_character (cast `/Game/Blueprints/Player/FirstPersonCharacter` (`GameplayStatics.GetPlayerCharacter` 0)))
      (`/Game/Blueprints/Player/FirstPersonCharacter.Water_Add_Hit_Failed` _asfirst_person_character)
      (else
        (set `self.Prefill Scale` _returnvalue_z)
        (bind (_direction _fill_amount) (`Timeline|Fill` :!via `PlayFromStart`)
          (:`Update`
            (bind _returnvalue (+ _fill_amount (`self.Prefill Scale`)))
            (if (> _returnvalue (`self.Max_Size`))
              (`self.SetActorScale3D` (`KismetMathLibrary.MakeVector` _returnvalue_x_2 _returnvalue_y_2 (`self.Max_Size`))) ; Min level
              (else
                (`self.SetActorScale3D` (`KismetMathLibrary.MakeVector` _returnvalue_x_3 _returnvalue_y_3 _returnvalue)) ; Drain
              ))))))))

(event `self.ReceiveAnyDamage`
  (params (Damage :type "Float (single-precision)") (DamageType :type "DamageType Object Reference") (InstigatedBy :type "Controller Object Reference") (DamageCauser :type "Actor Object Reference"))
  (bind (_returnvalue_x _returnvalue_y) (`KismetMathLibrary.BreakVector` (`SceneComponent.K2_GetComponentScale` (`self.Water`))))
  (bind (_returnvalue_x_2 _returnvalue_y_2) (`KismetMathLibrary.BreakVector` (`SceneComponent.K2_GetComponentScale` (`self.Water`))))
  (bind (_returnvalue_x_3 _returnvalue_y_3 _returnvalue_z) (`KismetMathLibrary.BreakVector` (`SceneComponent.K2_GetComponentScale` (`self.Water`))))
  (bind (_returnvalue_x_4 _returnvalue_y_4 _returnvalue_z_2) (`KismetMathLibrary.BreakVector` (`SceneComponent.K2_GetComponentScale` (`self.Water`))))
  ;[1 1 1] Drain Water
  (if (== (`GameplayStatics.GetObjectClass` DamageType) "/Game/Blueprints/Water_IO_block/WaterDrainDamage.WaterDrainDamage_C")
    (if (`KismetMathLibrary.NearlyEqual_FloatFloat` (`self.Min_Size`) _returnvalue_z_2 0.1)
      (bind _asfirst_person_character (cast `/Game/Blueprints/Player/FirstPersonCharacter` (`GameplayStatics.GetPlayerCharacter` 0)))
      (`/Game/Blueprints/Player/FirstPersonCharacter.Water_Subtract_Hit_Failed` _asfirst_person_character)
      (else
        (set `self.Prefill Scale` _returnvalue_z)
        (bind (_direction _drain_amount) (`Timeline|Drain_Timer` :!via `PlayFromStart`)
          (:`Update`
            (bind _returnvalue (- (`self.Prefill Scale`) _drain_amount))
            (if (< _returnvalue (`self.Min_Size`))
              (`self.SetActorScale3D` (`KismetMathLibrary.MakeVector` _returnvalue_x _returnvalue_y (`self.Min_Size`))) ; Min level
              (else
                (`self.SetActorScale3D` (`KismetMathLibrary.MakeVector` _returnvalue_x_2 _returnvalue_y_2 _returnvalue)) ; Drain
              ))))))))

(event `self.ReceiveActorBeginOverlap`
  (params (OtherActor :type "Actor Object Reference"))
  (set `self.IsDrowning` true)
  (`KismetSystemLibrary.Delay` 3.0 :!label _label)
  (if (`self.IsDrowning`)
    (`GameplayStatics.ApplyDamage` OtherActor 100.0)
    (goto _label)))

(event `self.ReceiveActorEndOverlap`
  (params (OtherActor :type "Actor Object Reference"))
  (set `self.IsDrowning` false))

(fn `UserConstructionScript`)